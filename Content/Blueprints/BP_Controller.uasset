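; BP_Controller is a controller Blueprint that shows short info or error messages on screen.
; On BeginPlay it creates a UI_DisplayMsg widget and adds it to the viewport.
; ShowinViewPort sets the widget's text and info/error flag, preferring the error message when one is given, then clears the text after a short delay.
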(event `self.ReceiveBeginPlay`
  (bind _returnvalue (`|CreateWidget` "/Game/Blueprints/UI_DisplayMsg.UI_DisplayMsg_C"))
  (bind _output_get (set `self.WidgetVar` _returnvalue))
  (`UserWidget.AddToViewport` _output_get 0))

(event `self.ShowInViewPort`
  (params (InfoMsg :type String) (ErrorMsg :type String))
  (if (`KismetStringLibrary.IsEmpty` ErrorMsg)
    (set `/Game/Blueprints/UI_DisplayMsg.displayMessage` InfoMsg (`self.WidgetVar`))
    (set `/Game/Blueprints/UI_DisplayMsg.isInfoMsg` true (`self.WidgetVar`))
    (`KismetSystemLibrary.Delay` 2.0)
    (set `/Game/Blueprints/UI_DisplayMsg.displayMessage` "" (`self.WidgetVar`))
    (else
      (set `/Game/Blueprints/UI_DisplayMsg.displayMessage` ErrorMsg (`self.WidgetVar`))
      (set `/Game/Blueprints/UI_DisplayMsg.isInfoMsg` false (`self.WidgetVar`))
      (`KismetSystemLibrary.Delay` 2.0)
      (set `/Game/Blueprints/UI_DisplayMsg.displayMessage` "" (`self.WidgetVar`)))))

(fn `UserConstructionScript`)